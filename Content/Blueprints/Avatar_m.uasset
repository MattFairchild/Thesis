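; Player avatar with VR and desktop cameras, plus character customization through hand-attached menus and a fingertip widget pointer.
; Tick moves the mesh under the HMD, turns the body from head yaw and hand-line alignment, and feeds head and hand transforms to the AnimBP.
; Height calibration derives a bone-stretch offset from HMD versus mesh height and re-grounds the mesh.
; Material and morph-target events set the appearance, which saves to and loads from a savegame slot.
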(event `Key|MotionController_Left_FaceButton3`
  (params (Key :type "Key Structure" :default "AnyKey"))
  ;[1 1 1] setup the right motion controller for widget interaction component
)

(event `Key|MotionController_Right_Trigger`
  (params (Key :type "Key Structure" :default "AnyKey"))
  (bind _righthandwidgetinteraction (`self.RightHandWidgetInteraction`))
  ;[1 1 1] setup the right motion controller for widget interaction component
  (:`Pressed`
    (`WidgetInteractionComponent.PressPointerKey` _righthandwidgetinteraction "LeftMouseButton"))
  (:`Released`
    (`WidgetInteractionComponent.ReleasePointerKey` _righthandwidgetinteraction "LeftMouseButton")))

(event `Key|MotionController_Left_FaceButton1`
  (params (Key :type "Key Structure" :default "AnyKey"))
  ;[1 1 1] setup the right motion controller for widget interaction component
  (:`Pressed`
    (set `self.rotateBodyWithHead` (not (`self.rotateBodyWithHead`)))))

(event `Key|MotionController_Right_FaceButton3`
  (params (Key :type "Key Structure" :default "AnyKey"))
  ;[1 1 1] setup the right motion controller for widget interaction component
  (:`Pressed`
    (`self.GetHeightDelta`)))

(event `savecurrentavatar`
  ;[1 1 1] save the current avatar appearance
  (bind _returnvalue (`GameplayStatics.CreateSaveGameObject` "/Game/Savegame/CharacterSavegame.CharacterSavegame_C"))
  (bind _ascharacter_savegame (cast `/Game/Savegame/CharacterSavegame` _returnvalue))
  (bind _output_get (set `self.Savegame` _ascharacter_savegame))
  (set `/Game/Savegame/CharacterSavegame.Playername` (`KismetTextLibrary.Conv_TextToString` (`self.Playername`)) _output_get)
  (set `/Game/Savegame/CharacterSavegame.SkinColor` (`self.SkinMatSavegame`) _output_get)
  (set `/Game/Savegame/CharacterSavegame.TorsoColor` (`self.TorsoMatSavegame`) _output_get)
  (set `/Game/Savegame/CharacterSavegame.LegsColor` (`self.LegsMatSavegame`) _output_get)
  (set `/Game/Savegame/CharacterSavegame.FeetColor` (`self.FeetMatSavegame`) _output_get)
  (set `/Game/Savegame/CharacterSavegame.HeadLengthMorph` (`self.HeadlengthMorph`) _output_get)
  (set `/Game/Savegame/CharacterSavegame.HeadSizeMorph` (`self.HeadsizeMorph`) _output_get)
  (set `/Game/Savegame/CharacterSavegame.NoseLengthMorph` (`self.NoselengthMorph`) _output_get)
  (set `/Game/Savegame/CharacterSavegame.BellySizeMorph` (`self.BellyMorph`) _output_get)
  (set `/Game/Savegame/CharacterSavegame.LegsThicknessMorph` (`self.LegsthicknessMorph`) _output_get)
  (`GameplayStatics.SaveGameToSlot` _output_get "savegame")
  (`KismetSystemLibrary.PrintString` "Wrote Savegame"))

(event `Key|MotionController_Left_FaceButton2`
  (params (Key :type "Key Structure" :default "AnyKey"))
  (bind _handmenu (`self.HandMenu`))
  (bind _returnvalue (`WidgetComponent.GetUserWidgetObject` (`self.HandMenu`)))
  ;[1 1 1] setup the right motion controller for widget interaction component
  (:`Pressed`
    (bind _returnvalue_2 (`|CreateWidget` "/Game/Widgets/CharacterCreation_Textures_Widget.CharacterCreation_Textures_Widget_C"))
    (`WidgetComponent.SetWidget` (`self.HandMenu`) _returnvalue_2)
    (`Widget.SetIsEnabled` _returnvalue true :!label _label)
    (`SceneComponent.SetVisibility` _handmenu true false))
  (:`Released`
    (`Widget.SetIsEnabled` _returnvalue false :!label _label_2)
    (`SceneComponent.SetVisibility` _handmenu false false)))

(event `Activate Cameras`
  ;[1 1 1] activate correct camera (either VR or desktop one)
  (bind _returnvalue (`HeadMountedDisplayFunctionLibrary.EnableHMD` true))
  (`ActorComponent.SetActive` (`self.VRCamera`) _returnvalue false)
  (`ActorComponent.SetActive` (`self.DesktopCamera`) (not _returnvalue) false))

(event `Key|MotionController_Left_FaceButton4`
  (params (Key :type "Key Structure" :default "AnyKey"))
  ;[1 1 1] setup the right motion controller for widget interaction component
  (:`Pressed`
    (bind _returnvalue (`|CreateWidget` "/Game/Widgets/CharacterCreation_Sliders_Widget.CharacterCreation_Sliders_Widget_C"))
    (`WidgetComponent.SetWidget` (`self.HandMenu`) _returnvalue)
    (goto _label))
  (:`Released`
    (goto _label_2)))

(event `self.ReceiveBeginPlay`
  (bind _returnvalue (`HeadMountedDisplayFunctionLibrary.IsHeadMountedDisplayEnabled`))
  (bind _handmenu (`self.HandMenu`))
  (bind _mesh (`self.Mesh`))
  ;[1 1 1] Begin Play
  (`self.Initialize`)
  (`self.Activate Cameras`)
  (`ActorComponent.SetActive` (`self.RightHandWidgetInteraction`) _returnvalue false)
  (if _returnvalue
    (`SkeletalMeshComponent.SetAnimInstanceClass` _mesh "/Game/Meshes/MultiTex/Avatar_m_AnimBlueprint.Avatar_m_AnimBlueprint_C")
    (else
      (`SkeletalMeshComponent.SetAnimInstanceClass` _mesh null)))
  (`self.Calculate Mesh height`)
  (set `self.DefaultMeshHeight` (`self.Meshheight`))
  (set `self.DefaultMeshTransform` (`SceneComponent.K2_GetComponentToWorld` (`self.Mesh`)))
  (`SceneComponent.K2_AttachToComponent` _handmenu (`self.Mesh`) "lefthand_socket" "SnapToTarget" "KeepRelative" "KeepRelative" true)
  (`SceneComponent.SetVisibility` _handmenu false false)
  (`SceneComponent.K2_AttachToComponent` (`self.RightHandWidgetInteraction`) (`self.Mesh`) "rightindexfinger_socket" "SnapToTarget" "KeepWorld" "KeepRelative" false))

(event `self.ReceiveTick`
  (params (DeltaSeconds :type "Float (single-precision)"))
  (bind _vrcamera (`self.VRCamera`))
  ;[1 1 1] Event Tick
  (set `self.Head Rotation` (`SceneComponent.K2_GetComponentRotation` _vrcamera))
  (set `self.Head Location` (`SceneComponent.K2_GetComponentLocation` _vrcamera))
  (if (`HeadMountedDisplayFunctionLibrary.IsHeadMountedDisplayEnabled`)
    (`self.Adjust Avatar Position to HMD position`))
  (`self.Update Anim BP`))

(event `Update Anim BP`
  (bind (_returnvalue_location _returnvalue_rotation) (`KismetMathLibrary.BreakTransform` (`SceneComponent.K2_GetComponentToWorld` (`self.Vive Hand Right`))))
  (bind (_returnvalue_location_2 _returnvalue_rotation_2) (`KismetMathLibrary.BreakTransform` (`SceneComponent.K2_GetComponentToWorld` (`self.Vive Hand Left`))))
  ;[1 1 1] update the Anim BP with values for hand position/rotation and head rotation
  (bind _asavatar_m_anim_blueprint (cast `/Game/Meshes/MultiTex/Avatar_m_AnimBlueprint` (`SkeletalMeshComponent.GetAnimInstance` (`self.Mesh`))))
  (`/Game/Meshes/MultiTex/Avatar_m_AnimBlueprint.UpdateHead` _asavatar_m_anim_blueprint (`self.Head Rotation`))
  (`/Game/Meshes/MultiTex/Avatar_m_AnimBlueprint.Set Right Hand Location` _asavatar_m_anim_blueprint _returnvalue_location)
  (`/Game/Meshes/MultiTex/Avatar_m_AnimBlueprint.Set Right Hand Rotation` _asavatar_m_anim_blueprint _returnvalue_rotation)
  (`/Game/Meshes/MultiTex/Avatar_m_AnimBlueprint.Set Left Hand Location` _asavatar_m_anim_blueprint _returnvalue_location_2)
  (`/Game/Meshes/MultiTex/Avatar_m_AnimBlueprint.Set Left Hand Rotation` _asavatar_m_anim_blueprint _returnvalue_rotation_2)
  (`/Game/Meshes/MultiTex/Avatar_m_AnimBlueprint.Set AdjustbonesHeight` _asavatar_m_anim_blueprint (`self.AdjustBonesHeight`)))

(event `GetHeightDelta`
  ;[1 1 1] get PLAYERHEIGHT / MESHHEIGHT / and the delta between them
  (`self.Calculate Playerheight`)
  (`self.Calculate Mesh height`)
  (set `self.AdjustBonesHeight` (- (`self.Playerheight`) (`self.Meshheight`)))
  (`self.AdjustMeshZPosition`))

(event `Calculate Mesh height`
  (bind _mesh (`self.Mesh`))
  (bind (_returnvalue_x _returnvalue_y _returnvalue_z) (`KismetMathLibrary.BreakVector` (`SceneComponent.GetSocketLocation` _mesh "root_socket")))
  (bind (_returnvalue_x_2 _returnvalue_y_2 _returnvalue_z_2) (`KismetMathLibrary.BreakVector` (`SceneComponent.GetSocketLocation` _mesh "head_socket")))
  ;[1 1 1] get PLAYERHEIGHT / MESHHEIGHT / and the delta between them
  ;;[1 1 1] get height of mesh from root- to head socket
  (set `self.Meshheight` (- _returnvalue_z_2 _returnvalue_z)))

(event `LoadSavegame`
  ;[1 1 1] load the saved appearance and apply it to the current one
  (bind _returnvalue (`GameplayStatics.LoadGameFromSlot` "savegame"))
  (bind _ascharacter_savegame (cast `/Game/Savegame/CharacterSavegame` _returnvalue))
  (bind _output_get (set `self.Savegame` _ascharacter_savegame))
  (`self.Change Skin Texture` (`/Game/Savegame/CharacterSavegame.SkinColor` _output_get))
  (`self.Change Torso Texture` (`/Game/Savegame/CharacterSavegame.TorsoColor` _output_get))
  (`self.Change Legs Texture` (`/Game/Savegame/CharacterSavegame.LegsColor` _output_get))
  (`self.Change Feet Texture` (`/Game/Savegame/CharacterSavegame.FeetColor` _output_get))
  (`self.change head size morph target` (`/Game/Savegame/CharacterSavegame.HeadSizeMorph` _output_get))
  (`self.change head length morph target` (`/Game/Savegame/CharacterSavegame.HeadLengthMorph` _output_get))
  (`self.change nose morph target` (`/Game/Savegame/CharacterSavegame.NoseLengthMorph` _output_get))
  (`self.change belly size morph target` (`/Game/Savegame/CharacterSavegame.BellySizeMorph` _output_get))
  (`self.change leg thickness morph target` (`/Game/Savegame/CharacterSavegame.LegsThicknessMorph` _output_get)))

(event `Calculate Playerheight`
  (bind (_head_location_x _head_location_y _head_location_z) (`KismetMathLibrary.BreakVector` (`self.Head Location`)))
  ;[1 1 1] get PLAYERHEIGHT / MESHHEIGHT / and the delta between them
  ;;[1 1 1] height of the HMD
  (set `self.Playerheight` (- _head_location_z 14.0)))

(event `Key|ö`
  (params (Key :type "Key Structure" :default "AnyKey"))
  (:`Pressed`
    (bind _output_get (set `self.AdjustBonesHeight` (+ (`self.AdjustBonesHeight`) 5.0)))
    (`KismetSystemLibrary.PrintString` (`KismetStringLibrary.Conv_DoubleToString` _output_get))
    (`self.AdjustMeshZPosition` :!label _label_3)))

(event `Key|ä`
  (params (Key :type "Key Structure" :default "AnyKey"))
  (:`Pressed`
    (bind _output_get (set `self.AdjustBonesHeight` (- (`self.AdjustBonesHeight`) 5.0)))
    (`KismetSystemLibrary.PrintString` (`KismetStringLibrary.Conv_DoubleToString` _output_get))
    (goto _label_3)))

(event `Adjust Avatar Position to HMD position`
  ;[1 1 1] Adjust the avatar as a whole to move with the HMD
  (`self.SetMeshRotation`))

(event `AdjustMeshZPosition`
  (bind _mesh (`self.Mesh`))
  (bind (_returnvalue_x _returnvalue_y) (`KismetMathLibrary.BreakVector` (`SceneComponent.K2_GetComponentLocation` _mesh)))
  ;[1 1 1] adjust mesh height to have it stand on ground after stretching it via "adjustbonesheight" and ANimBP
  (`SceneComponent.K2_SetWorldLocation` _mesh (`KismetMathLibrary.MakeVector` _returnvalue_x _returnvalue_y (+ (.z (.location (`self.DefaultMeshTransform`))) (* (`self.AdjustBonesHeight`) 0.4))) false false))

(event `InputAxis|MoveRight`
  (params (AxisValue :type "Float (single-precision)"))
  (bind _mesh (`self.Mesh`))
  (bind (_returnvalue_roll _returnvalue_pitch _returnvalue_yaw) (`KismetMathLibrary.BreakRotator` (`SceneComponent.K2_GetComponentRotation` _mesh)))
  ;[1 1 1] rotate avatar on pressing A or D (set in input project settings)
  (`SceneComponent.K2_SetWorldRotation` _mesh (`KismetMathLibrary.MakeRotator` 0.0 0.0 (- _returnvalue_yaw AxisValue)) false false))

(event `change nose morph target`
  (params (NewParam :type "Float (double-precision)"))
  ;[1 1 1] change morph targets
  (`SkeletalMeshComponent.SetMorphTarget` (`self.Mesh`) "GrowNose" NewParam true)
  (set `self.NoselengthMorph` NewParam))

(event `Key|Q`
  (params (Key :type "Key Structure" :default "AnyKey"))
  ;[1 1 1] adjust camer location
  (:`Pressed`
    (bind _output_get (set `self.adjustHeight` (+ (`self.adjustHeight`) 5.0)))
    (`KismetSystemLibrary.PrintString` (`KismetStringLibrary.Conv_DoubleToString` _output_get))))

(event `Change Skin Texture`
  (params (NewParam :type "MaterialInterface Object Reference"))
  ;[1 1 1] change Textures
  ;;[1 1 1] change skin texture
  (`PrimitiveComponent.SetMaterial` (`self.Mesh`) 2 NewParam)
  (set `self.SkinMatSavegame` NewParam))

(event `Key|W`
  (params (Key :type "Key Structure" :default "AnyKey"))
  ;[1 1 1] adjust camer location
  (:`Pressed`
    (bind _output_get (set `self.adjustHeight` (- (`self.adjustHeight`) 5.0)))
    (`KismetSystemLibrary.PrintString` (`KismetStringLibrary.Conv_DoubleToString` _output_get))))

(event `change head size morph target`
  (params (NewParam :type "Float (double-precision)"))
  ;[1 1 1] change morph targets
  (`SkeletalMeshComponent.SetMorphTarget` (`self.Mesh`) "HeadSize" NewParam true)
  (set `self.HeadsizeMorph` NewParam))

(event `Key|E`
  (params (Key :type "Key Structure" :default "AnyKey"))
  ;[1 1 1] adjust camer location
  (:`Pressed`
    (bind _output_get (set `self.Adjust Sideways` (+ (`self.Adjust Sideways`) 3.0)))
    (`KismetSystemLibrary.PrintString` (`KismetStringLibrary.Conv_DoubleToString` _output_get))))

(event `Change Torso Texture`
  (params (NewParam :type "MaterialInterface Object Reference"))
  ;[1 1 1] change Textures
  ;;[1 1 1] change torso teyture
  (`PrimitiveComponent.SetMaterial` (`self.Mesh`) 1 NewParam)
  (set `self.TorsoMatSavegame` NewParam))

(event `change belly size morph target`
  (params (NewParam :type "Float (double-precision)"))
  ;[1 1 1] change morph targets
  (`SkeletalMeshComponent.SetMorphTarget` (`self.Mesh`) "Belly" NewParam true)
  (set `self.BellyMorph` NewParam))

(event `Key|R`
  (params (Key :type "Key Structure" :default "AnyKey"))
  ;[1 1 1] adjust camer location
  (:`Pressed`
    (bind _output_get (set `self.Adjust Sideways` (+ (`self.Adjust Sideways`) -3.0)))
    (`KismetSystemLibrary.PrintString` (`KismetStringLibrary.Conv_DoubleToString` _output_get))))

(event `Key|T`
  (params (Key :type "Key Structure" :default "AnyKey"))
  ;[1 1 1] adjust camer location
  (:`Pressed`
    (bind _output_get (set `self.Adjust Forward` (+ (`self.Adjust Forward`) 3.0)))
    (`KismetSystemLibrary.PrintString` (`KismetStringLibrary.Conv_DoubleToString` _output_get))))

(event `Change Legs Texture`
  (params (NewParam :type "MaterialInterface Object Reference"))
  ;[1 1 1] change Textures
  ;;[1 1 1] change legs texture
  (`PrimitiveComponent.SetMaterial` (`self.Mesh`) 0 NewParam)
  (set `self.LegsMatSavegame` NewParam))

(event `change leg thickness morph target`
  (params (NewParam :type "Float (double-precision)"))
  ;[1 1 1] change morph targets
  (`SkeletalMeshComponent.SetMorphTarget` (`self.Mesh`) "Legs" NewParam true)
  (set `self.LegsthicknessMorph` NewParam))

(event `Key|Z`
  (params (Key :type "Key Structure" :default "AnyKey"))
  ;[1 1 1] adjust camer location
  (:`Pressed`
    (bind _output_get (set `self.Adjust Forward` (+ (`self.Adjust Forward`) -3.0)))
    (`KismetSystemLibrary.PrintString` (`KismetStringLibrary.Conv_DoubleToString` _output_get))))

(event `change head length morph target`
  (params (NewParam :type "Float (double-precision)"))
  ;[1 1 1] change morph targets
  (`SkeletalMeshComponent.SetMorphTarget` (`self.Mesh`) "headLength" NewParam true)
  (set `self.NoselengthMorph` NewParam))

(event `Change Feet Texture`
  (params (NewParam :type "MaterialInterface Object Reference"))
  ;[1 1 1] change Textures
  ;;[1 1 1] change feet texture
  (`PrimitiveComponent.SetMaterial` (`self.Mesh`) 3 NewParam)
  (set `self.FeetMatSavegame` NewParam))

(event `ChangePlayername`
  (params (`new name` :type Text))
  ;[1 1 1] Set the playername
  (set `self.Playername` `new name`))

(fn `CheckForBodyRotationTrigger`
  (returns (Yaw :type "Float (double-precision)") (triggered :type Boolean))
  (bind (_returnvalue_roll _returnvalue_pitch _returnvalue_yaw) (`KismetMathLibrary.BreakRotator` (`SceneComponent.K2_GetComponentRotation` (`self.VRCamera`))))
  (bind (_returnvalue_x _returnvalue_y) (`KismetMathLibrary.BreakVector` (`SceneComponent.GetForwardVector` (`self.VRCamera`))))
  (bind _normalizedforward (`self.GetHandsFoward`))
  (bind _angle (`self.GetAngle0-360` _normalizedforward (`KismetMathLibrary.Normal` (`KismetMathLibrary.MakeVector` _returnvalue_x _returnvalue_y))))
  (if (and (< _angle 10.0) (> _angle -10.0))
    (return _returnvalue_yaw true)
    (else
      (return 0.0 false))))

(fn `DrawDebugLinesHandsAndFace`
  (bind _returnvalue (`SceneComponent.GetSocketLocation` (`self.Mesh`) "spine_socket"))
  (bind (_returnvalue_x _returnvalue_y) (`KismetMathLibrary.BreakVector` (`SceneComponent.GetForwardVector` (`self.VRCamera`))))
  (`KismetSystemLibrary.DrawDebugLine` _returnvalue (+ _returnvalue (* (`self.HandsFoward`) 1000.0)) (struct :`R` 0.975 :`B` 0.870857 :`A` 1.0) 0.0 1.0)
  (`KismetSystemLibrary.DrawDebugLine` _returnvalue (+ _returnvalue (`KismetMathLibrary.MakeVector` (* _returnvalue_x 1000.0) (* _returnvalue_y 1000.0))) (struct :`G` 1.0 :`B` 0.944436 :`A` 1.0) 0.0 1.0))

(fn `GetAngle0-360`
  (params (vec1 :type "Vector Structure") (vec2 :type "Vector Structure"))
  (returns (angle :type "Float (double-precision)"))
  (return (- (`KismetMathLibrary.DegAtan2` vec1_Y vec1_X) (`KismetMathLibrary.DegAtan2` vec2_Y vec2_X))))

(fn `GetHandsFoward`
  (returns (NormalizedForward :type "Vector Structure"))
  (bind (_returnvalue_x _returnvalue_y) (`KismetMathLibrary.BreakVector` (- (`SceneComponent.K2_GetComponentLocation` (`self.Vive Hand Left`)) (`SceneComponent.K2_GetComponentLocation` (`self.Vive Hand Right`)))))
  (bind _returnvalue (`KismetMathLibrary.Normal` (`KismetMathLibrary.MakeVector` (* _returnvalue_y -1.0) _returnvalue_x)))
  (set `self.HandsFoward` _returnvalue)
  (return _returnvalue))

(fn `Initialize`
  (bind (_returnvalue_x _returnvalue_y) (`KismetMathLibrary.BreakVector` (`SceneComponent.K2_GetComponentLocation` (`self.Vive Hand Left`))))
  (bind (_returnvalue_x_2 _returnvalue_y_2) (`KismetMathLibrary.BreakVector` (`SceneComponent.K2_GetComponentLocation` (`self.Mesh`))))
  (bind (_returnvalue_x_3 _returnvalue_y_3) (`KismetMathLibrary.BreakVector` (`SceneComponent.K2_GetComponentLocation` (`self.Vive Hand Right`))))
  (bind _returnvalue (`KismetMathLibrary.MakeVector` _returnvalue_x_2 _returnvalue_y_2))
  (set `self.rightHand_Direction` (`KismetMathLibrary.Normal` (- (`KismetMathLibrary.MakeVector` _returnvalue_x_3 _returnvalue_y_3) _returnvalue)))
  (set `self.leftHand_Direction` (`KismetMathLibrary.Normal` (- (`KismetMathLibrary.MakeVector` _returnvalue_x _returnvalue_y) _returnvalue))))

(fn `SetMeshRotation`
  (locals (bodyRotation :type "Float (double-precision)") (ForwardDelta :type "Float (double-precision)"))
  (bind (_returnvalue_x _returnvalue_y _returnvalue_z) (`KismetMathLibrary.BreakVector` (`SceneComponent.K2_GetComponentLocation` (`self.Mesh`))))
  (bind (_returnvalue_roll _returnvalue_pitch _returnvalue_yaw) (`KismetMathLibrary.BreakRotator` (`SceneComponent.K2_GetComponentRotation` (`self.Mesh`))))
  (bind (_returnvalue_x_2 _returnvalue_y_2) (`KismetMathLibrary.BreakVector` (`SceneComponent.K2_GetComponentLocation` (`self.VRCamera`))))
  (bind (_returnvalue_roll_2 _returnvalue_pitch_2 _returnvalue_yaw_2) (`KismetMathLibrary.BreakRotator` (`KismetMathLibrary.MakeRotator` _returnvalue_roll _returnvalue_pitch (- (`local.bodyRotation`) 90.0))))
  (`SceneComponent.K2_SetWorldLocation` (`self.Mesh`) (+ (`KismetMathLibrary.MakeVector` _returnvalue_x_2 _returnvalue_y_2 _returnvalue_z) (* (`SceneComponent.GetRightVector` (`self.Mesh`)) -13.0)) false false)
  ;[1 1 1] Roatet the body only when the head is rotated more than 90 degrees in either direction
  (bind _angle (`self.GetAngle0-360` (`SceneComponent.GetForwardVector` (`self.VRCamera`)) (`SceneComponent.GetRightVector` (`self.Mesh`))))
  (bind _output_get (set `local.ForwardDelta` _angle))
  (if (> _output_get 90.0)
    (set `local.bodyRotation` (- (`local.ForwardDelta`) 90.0))
    (elif (< (`local.ForwardDelta`) -90.0)
      (set `local.bodyRotation` (+ (`local.ForwardDelta`) 90.0))))
  (`SceneComponent.K2_AddWorldRotation` (`self.Mesh`) (`KismetMathLibrary.MakeRotator` 0.0 0.0 (`local.bodyRotation`)) false false)
  (`self.DrawDebugLinesHandsAndFace`)
  (bind (_yaw _triggered) (`self.CheckForBodyRotationTrigger`))
  (set `local.bodyRotation` _yaw)
  (if _triggered
    (`SceneComponent.K2_SetWorldRotation` (`self.Mesh`) (`KismetMathLibrary.RInterpTo` (`KismetMathLibrary.MakeRotator` _returnvalue_roll _returnvalue_pitch _returnvalue_yaw) (`KismetMathLibrary.MakeRotator` _returnvalue_roll_2 _returnvalue_pitch_2 _returnvalue_yaw_2) (`GameplayStatics.GetWorldDeltaSeconds`) 0.0) false false)))

(fn `UserConstructionScript`)