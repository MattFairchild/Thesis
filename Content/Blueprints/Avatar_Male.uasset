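; Customizable male avatar for VR with desktop fallback, embodying the player through HMD and motion controllers.
; In VR, Tick moves the mesh under the headset with key-tuned offsets and feeds head and hand transforms to Avatar_AnimBP, plus a calibratable bone height.
; Change events apply body-part materials and morph targets and cache them for CharacterSavegame, which saves appearance and name and reloads appearance.
; The right trigger drives widget interaction.
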(event `savecurrentavatar`
  ;[1 1 1] save the current avatar appearance
  (bind _returnvalue (`GameplayStatics.CreateSaveGameObject` "/Game/Savegame/CharacterSavegame.CharacterSavegame_C"))
  (bind _ascharacter_savegame (cast `/Game/Savegame/CharacterSavegame` _returnvalue))
  (bind _output_get (set `self.Savegame` _ascharacter_savegame))
  (set `/Game/Savegame/CharacterSavegame.Playername` (`KismetTextLibrary.Conv_TextToString` (`self.Playername`)) _output_get)
  (set `/Game/Savegame/CharacterSavegame.SkinColor` (`self.SkinMatSavegame`) _output_get)
  (set `/Game/Savegame/CharacterSavegame.TorsoColor` (`self.TorsoMatSavegame`) _output_get)
  (set `/Game/Savegame/CharacterSavegame.LegsColor` (`self.LegsMatSavegame`) _output_get)
  (set `/Game/Savegame/CharacterSavegame.FeetColor` (`self.FeetMatSavegame`) _output_get)
  (set `/Game/Savegame/CharacterSavegame.HeadLengthMorph` (`self.HeadlengthMorph`) _output_get)
  (set `/Game/Savegame/CharacterSavegame.HeadSizeMorph` (`self.HeadsizeMorph`) _output_get)
  (set `/Game/Savegame/CharacterSavegame.NoseLengthMorph` (`self.NoselengthMorph`) _output_get)
  (set `/Game/Savegame/CharacterSavegame.BellySizeMorph` (`self.BellyMorph`) _output_get)
  (set `/Game/Savegame/CharacterSavegame.LegsThicknessMorph` (`self.LegsthicknessMorph`) _output_get)
  (`GameplayStatics.SaveGameToSlot` _output_get "savegame")
  (`KismetSystemLibrary.PrintString` "Wrote Savegame"))

(event `Activate Cameras`
  ;[1 1 1] activate correct camera (either VR or desktop one)
  (bind _returnvalue (`HeadMountedDisplayFunctionLibrary.EnableHMD` true))
  (`ActorComponent.SetActive` (`self.VRCamera`) _returnvalue false)
  (`ActorComponent.SetActive` (`self.DesktopCamera`) (not _returnvalue) false))

(event `Key|MotionController_Right_Trigger`
  (params (Key :type "Key Structure" :default "AnyKey"))
  (bind _righthandwidgetinteraction (`self.RightHandWidgetInteraction`))
  ;[1 1 1] setup the right motion controller for widget interaction component
  (:`Pressed`
    (`WidgetInteractionComponent.PressPointerKey` _righthandwidgetinteraction "LeftMouseButton"))
  (:`Released`
    (`WidgetInteractionComponent.ReleasePointerKey` _righthandwidgetinteraction "LeftMouseButton")))

(event `self.ReceiveBeginPlay`
  (bind _returnvalue (`HeadMountedDisplayFunctionLibrary.IsHeadMountedDisplayEnabled`))
  (bind _mesh (`self.Mesh`))
  ;[1 1 1] Begin Play
  (`self.Activate Cameras`)
  (`ActorComponent.SetActive` (`self.RightHandWidgetInteraction`) _returnvalue false)
  (if _returnvalue
    (`SkeletalMeshComponent.SetAnimInstanceClass` _mesh "/Game/Meshes/AvatarMale/Avatar_AnimBP.Avatar_AnimBP_C")
    (else
      (`SkeletalMeshComponent.SetAnimInstanceClass` _mesh null))))

(event `Key|MotionController_Left_Trigger`
  (params (Key :type "Key Structure" :default "AnyKey"))
  ;[1 1 1] setup the right motion controller for widget interaction component
  (:`Pressed`
    (`self.GetHeadDelta`)))

(event `self.ReceiveTick`
  (params (DeltaSeconds :type "Float (single-precision)"))
  (bind _vrcamera (`self.VRCamera`))
  ;[1 1 1] Event Tick
  (set `self.Head Rotation` (`SceneComponent.K2_GetComponentRotation` _vrcamera))
  (set `self.Head Location` (`SceneComponent.K2_GetComponentLocation` _vrcamera))
  (if (`HeadMountedDisplayFunctionLibrary.IsHeadMountedDisplayEnabled`)
    (`self.Adjust Avatar Position to HMD position`))
  (`self.Update Anim BP`))

(event `Update Anim BP`
  (bind (_returnvalue_location _returnvalue_rotation) (`KismetMathLibrary.BreakTransform` (`SceneComponent.K2_GetComponentToWorld` (`self.Vive Hand Right`))))
  (bind (_returnvalue_location_2 _returnvalue_rotation_2) (`KismetMathLibrary.BreakTransform` (`SceneComponent.K2_GetComponentToWorld` (`self.Vive Hand Left`))))
  ;[1 1 1] update the Anim BP with values for hand position/rotation and head rotation
  (bind _asavatar_anim_bp (cast `/Game/Meshes/AvatarMale/Avatar_AnimBP` (`SkeletalMeshComponent.GetAnimInstance` (`self.Mesh`))))
  (set `/Game/Meshes/AvatarMale/Avatar_AnimBP.HeadRotation_Target` (`self.Head Rotation`) _asavatar_anim_bp)
  (set `/Game/Meshes/AvatarMale/Avatar_AnimBP.RighthandLocation_Target` _returnvalue_location _asavatar_anim_bp)
  (set `/Game/Meshes/AvatarMale/Avatar_AnimBP.RighthandRotation_Target` _returnvalue_rotation _asavatar_anim_bp)
  (set `/Game/Meshes/AvatarMale/Avatar_AnimBP.LefthandLocation_Target` _returnvalue_location_2 _asavatar_anim_bp)
  (set `/Game/Meshes/AvatarMale/Avatar_AnimBP.LefthandRotation_Target` _returnvalue_rotation_2 _asavatar_anim_bp)
  (set `/Game/Meshes/AvatarMale/Avatar_AnimBP.AdjustBoneHeight` (`self.AdjustBonesHeight`) _asavatar_anim_bp))

(event `GetHeadDelta`
  (bind (_head_location_x _head_location_y _head_location_z) (`KismetMathLibrary.BreakVector` (`self.Head Location`)))
  (bind (_returnvalue_x _returnvalue_y _returnvalue_z) (`KismetMathLibrary.BreakVector` (`SceneComponent.GetSocketLocation` (`self.Mesh`) "head_socket")))
  (set `self.AdjustBonesHeight` (- _head_location_z _returnvalue_z)))

(event `LoadSavegame`
  ;[1 1 1] load the saved appearance and apply it to the current one
  (bind _returnvalue (`GameplayStatics.LoadGameFromSlot` "savegame"))
  (bind _ascharacter_savegame (cast `/Game/Savegame/CharacterSavegame` _returnvalue))
  (bind _output_get (set `self.Savegame` _ascharacter_savegame))
  (`self.Change Skin Texture` (`/Game/Savegame/CharacterSavegame.SkinColor` _output_get))
  (`self.Change Torso Texture` (`/Game/Savegame/CharacterSavegame.TorsoColor` _output_get))
  (`self.Change Legs Texture` (`/Game/Savegame/CharacterSavegame.LegsColor` _output_get))
  (`self.Change Feet Texture` (`/Game/Savegame/CharacterSavegame.FeetColor` _output_get))
  (`self.change head size morph target` (`/Game/Savegame/CharacterSavegame.HeadSizeMorph` _output_get))
  (`self.change head length morph target` (`/Game/Savegame/CharacterSavegame.HeadLengthMorph` _output_get))
  (`self.change nose morph target` (`/Game/Savegame/CharacterSavegame.NoseLengthMorph` _output_get))
  (`self.change belly size morph target` (`/Game/Savegame/CharacterSavegame.BellySizeMorph` _output_get))
  (`self.change leg thickness morph target` (`/Game/Savegame/CharacterSavegame.LegsThicknessMorph` _output_get)))

(event `Key|ö`
  (params (Key :type "Key Structure" :default "AnyKey"))
  (:`Pressed`
    (set `self.AdjustBonesHeight` (+ (`self.AdjustBonesHeight`) 5.0))))

(event `Key|ä`
  (params (Key :type "Key Structure" :default "AnyKey"))
  (:`Pressed`
    (set `self.AdjustBonesHeight` (- (`self.AdjustBonesHeight`) 5.0))))

(event `Adjust Avatar Position to HMD position`
  (bind (_returnvalue_x _returnvalue_y _returnvalue_z) (`KismetMathLibrary.BreakVector` (`SceneComponent.K2_GetComponentLocation` (`self.VRCamera`))))
  ;[1 1 1] Adjust the avatar as a whole to move with the HMD
  (`SceneComponent.K2_SetWorldLocation` (`self.Mesh`) (`KismetMathLibrary.MakeVector` (+ _returnvalue_x (`self.Adjust Forward`)) (+ _returnvalue_y (`self.Adjust Sideways`)) (- _returnvalue_z (`self.adjustHeight`))) false false))

(event `InputAxis|MoveRight`
  (params (AxisValue :type "Float (single-precision)"))
  (bind _mesh (`self.Mesh`))
  (bind (_returnvalue_roll _returnvalue_pitch _returnvalue_yaw) (`KismetMathLibrary.BreakRotator` (`SceneComponent.K2_GetComponentRotation` _mesh)))
  ;[1 1 1] rotate avatar on pressing A or D (set in input project settings)
  (`SceneComponent.K2_SetWorldRotation` _mesh (`KismetMathLibrary.MakeRotator` 0.0 0.0 (- _returnvalue_yaw AxisValue)) false false))

(event `change nose morph target`
  (params (NewParam :type "Float (double-precision)"))
  ;[1 1 1] change morph targets
  (`SkeletalMeshComponent.SetMorphTarget` (`self.Mesh`) "GrowNose" NewParam true)
  (set `self.NoselengthMorph` NewParam))

(event `Key|Q`
  (params (Key :type "Key Structure" :default "AnyKey"))
  ;[1 1 1] adjust camer location
  (:`Pressed`
    (bind _output_get (set `self.adjustHeight` (+ (`self.adjustHeight`) 5.0)))
    (`KismetSystemLibrary.PrintString` (`KismetStringLibrary.Conv_DoubleToString` _output_get))))

(event `Change Skin Texture`
  (params (NewParam :type "MaterialInterface Object Reference"))
  ;[1 1 1] change Textures
  ;;[1 1 1] change skin texture
  (`PrimitiveComponent.SetMaterial` (`self.Mesh`) 2 NewParam)
  (set `self.SkinMatSavegame` NewParam))

(event `Key|W`
  (params (Key :type "Key Structure" :default "AnyKey"))
  ;[1 1 1] adjust camer location
  (:`Pressed`
    (bind _output_get (set `self.adjustHeight` (- (`self.adjustHeight`) 5.0)))
    (`KismetSystemLibrary.PrintString` (`KismetStringLibrary.Conv_DoubleToString` _output_get))))

(event `change head size morph target`
  (params (NewParam :type "Float (double-precision)"))
  ;[1 1 1] change morph targets
  (`SkeletalMeshComponent.SetMorphTarget` (`self.Mesh`) "HeadSize" NewParam true)
  (set `self.HeadsizeMorph` NewParam))

(event `Key|E`
  (params (Key :type "Key Structure" :default "AnyKey"))
  ;[1 1 1] adjust camer location
  (:`Pressed`
    (bind _output_get (set `self.Adjust Sideways` (+ (`self.Adjust Sideways`) 3.0)))
    (`KismetSystemLibrary.PrintString` (`KismetStringLibrary.Conv_DoubleToString` _output_get))))

(event `Change Torso Texture`
  (params (NewParam :type "MaterialInterface Object Reference"))
  ;[1 1 1] change Textures
  ;;[1 1 1] change torso teyture
  (`PrimitiveComponent.SetMaterial` (`self.Mesh`) 1 NewParam)
  (set `self.TorsoMatSavegame` NewParam))

(event `change belly size morph target`
  (params (NewParam :type "Float (double-precision)"))
  ;[1 1 1] change morph targets
  (`SkeletalMeshComponent.SetMorphTarget` (`self.Mesh`) "Belly" NewParam true)
  (set `self.BellyMorph` NewParam))

(event `Key|R`
  (params (Key :type "Key Structure" :default "AnyKey"))
  ;[1 1 1] adjust camer location
  (:`Pressed`
    (bind _output_get (set `self.Adjust Sideways` (+ (`self.Adjust Sideways`) -3.0)))
    (`KismetSystemLibrary.PrintString` (`KismetStringLibrary.Conv_DoubleToString` _output_get))))

(event `Key|T`
  (params (Key :type "Key Structure" :default "AnyKey"))
  ;[1 1 1] adjust camer location
  (:`Pressed`
    (bind _output_get (set `self.Adjust Forward` (+ (`self.Adjust Forward`) 3.0)))
    (`KismetSystemLibrary.PrintString` (`KismetStringLibrary.Conv_DoubleToString` _output_get))))

(event `Change Legs Texture`
  (params (NewParam :type "MaterialInterface Object Reference"))
  ;[1 1 1] change Textures
  ;;[1 1 1] change legs texture
  (`PrimitiveComponent.SetMaterial` (`self.Mesh`) 0 NewParam)
  (set `self.LegsMatSavegame` NewParam))

(event `change leg thickness morph target`
  (params (NewParam :type "Float (double-precision)"))
  ;[1 1 1] change morph targets
  (`SkeletalMeshComponent.SetMorphTarget` (`self.Mesh`) "Legs" NewParam true)
  (set `self.LegsthicknessMorph` NewParam))

(event `Key|Z`
  (params (Key :type "Key Structure" :default "AnyKey"))
  ;[1 1 1] adjust camer location
  (:`Pressed`
    (bind _output_get (set `self.Adjust Forward` (+ (`self.Adjust Forward`) -3.0)))
    (`KismetSystemLibrary.PrintString` (`KismetStringLibrary.Conv_DoubleToString` _output_get))))

(event `change head length morph target`
  (params (NewParam :type "Float (double-precision)"))
  ;[1 1 1] change morph targets
  (`SkeletalMeshComponent.SetMorphTarget` (`self.Mesh`) "headLength" NewParam true)
  (set `self.NoselengthMorph` NewParam))

(event `Change Feet Texture`
  (params (NewParam :type "MaterialInterface Object Reference"))
  ;[1 1 1] change Textures
  ;;[1 1 1] change feet texture
  (`PrimitiveComponent.SetMaterial` (`self.Mesh`) 3 NewParam)
  (set `self.FeetMatSavegame` NewParam))

(event `ChangePlayername`
  (params (`new name` :type Text))
  ;[1 1 1] Set the playername
  (set `self.Playername` `new name`))

(fn `UserConstructionScript`)