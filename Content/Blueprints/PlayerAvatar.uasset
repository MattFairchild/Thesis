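; Player avatar for VR or desktop play, with a customizable body and a character creation HUD shown at BeginPlay.
; Each tick moves the mesh to the VR camera plus key-adjustable offsets and feeds head rotation and Vive hand transforms to the animation Blueprint.
; Events set morph targets for body shape, swap skin, torso, legs and feet materials, and scale the mesh.
; An enableHMD flag selects the active camera.
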(event Custom|Update%20Anim%20BP
  (bind _vive_hand_right (Variables|Default|GetVive%20Hand%20Right))
  (bind _vive_hand_left (Variables|Default|GetVive%20Hand%20Left))
  (bind _returnvalue (Transformation|GetWorldTransform _vive_hand_right))
  (bind _returnvalue_2 (Transformation|GetWorldTransform _vive_hand_left))
  ;[1 1 1] update the Anim BP with values for hand position/rotation and head rotation
  (bind _asmulti_texture_anim_blueprint (Utilities|Casting|CastTomultiTexture_AnimBlueprint (Components|SkeletalMesh|GetAnimInstance (Variables|Character|GetMesh))))
  (Default|UpdateHead _asmulti_texture_anim_blueprint (Variables|Default|GetHead%20Rotation))
  (Default|SetRightHandLocation _asmulti_texture_anim_blueprint (.location _returnvalue))
  (Default|SetRightHandRotation _asmulti_texture_anim_blueprint (.rotation _returnvalue))
  (Default|SetLeftHandLocation _asmulti_texture_anim_blueprint (.location _returnvalue_2))
  (Default|SetLeftHandRotation _asmulti_texture_anim_blueprint (.rotation _returnvalue_2)))

(event Custom|Change%20Torso%20Texture
  (params (NewParam :type Material%20Interface%20Object%20Reference))
  ;[1 1 1] change Textures
  ;;[1 1 1] change torso teyture
  (Rendering|Material|SetMaterial (Variables|Character|GetMesh) 1 NewParam))

(event Custom|Change%20Feet%20Texture
  (params (NewParam :type Material%20Interface%20Object%20Reference))
  ;[1 1 1] change Textures
  ;;[1 1 1] change feet texture
  (Rendering|Material|SetMaterial (Variables|Character|GetMesh) 3 NewParam))

(event Custom|Change%20Skin%20Texture
  (params (NewParam :type Material%20Interface%20Object%20Reference))
  ;[1 1 1] change Textures
  ;;[1 1 1] change skin texture
  (Rendering|Material|SetMaterial (Variables|Character|GetMesh) 2 NewParam))

(event Custom|Change%20Legs%20Texture
  (params (NewParam :type Material%20Interface%20Object%20Reference))
  ;[1 1 1] change Textures
  ;;[1 1 1] change legs texture
  (Rendering|Material|SetMaterial (Variables|Character|GetMesh) 0 NewParam))

(event Custom|change%20nose%20morph%20target
  (params (NewParam :type Float%20%28single-precision%29))
  ;[1 1 1] change morph targets
  (Components|SkeletalMesh|SetMorphTarget (Variables|Character|GetMesh) "GrowNose" NewParam true))

(event Custom|Adjust%20Avatar%20Position%20to%20HMD%20position
  (bind _vrcamera (Variables|Default|GetVRCamera))
  (bind _returnvalue (Transformation|GetWorldLocation _vrcamera))
  ;[1 1 1] Adjust the avatar as a whole to move with the HMD
  (Transformation|SetWorldLocation (Variables|Character|GetMesh) (Math|Vector|MakeVector (+ (.x _returnvalue) (Variables|Default|GetAdjust%20Forward)) (+ (.y _returnvalue) (Variables|Default|GetAdjust%20Sideways)) (- (.z _returnvalue) (Variables|Default|GetadjustHeight))) false false))

(event Custom|change%20head%20size%20morph%20target
  (params (NewParam :type Float%20%28single-precision%29))
  ;[1 1 1] change morph targets
  (Components|SkeletalMesh|SetMorphTarget (Variables|Character|GetMesh) "HeadSize" NewParam true))

(event Custom|Activate%20Cameras
  ;[1 1 1] activate correct camera (either VR or desktop one)
  (Components|Activation|SetActive (Variables|Default|GetVRCamera) (stale _returnvalue) false)
  (Components|Activation|SetActive (Variables|Default|GetDesktopCamera) (not (stale _returnvalue)) false))

(event Custom|change%20belly%20size%20morph%20target
  (params (NewParam :type Float%20%28single-precision%29))
  ;[1 1 1] change morph targets
  (Components|SkeletalMesh|SetMorphTarget (Variables|Character|GetMesh) "Belly" NewParam true))

(event Custom|change%20head%20length%20morph%20target
  (params (NewParam :type Float%20%28single-precision%29))
  ;[1 1 1] change morph targets
  (Components|SkeletalMesh|SetMorphTarget (Variables|Character|GetMesh) "headLength" NewParam true))

(event Custom|change%20leg%20thickness%20morph%20target
  (params (NewParam :type Float%20%28single-precision%29))
  ;[1 1 1] change morph targets
  (Components|SkeletalMesh|SetMorphTarget (Variables|Character|GetMesh) "Legs" NewParam true))

(event Custom|change%20arm%20smaller%20morph%20target
  (params (NewParam :type Float%20%28single-precision%29))
  ;[1 1 1] change morph targets
  (Components|SkeletalMesh|SetMorphTarget (Variables|Character|GetMesh) "Armlengthsmaller" NewParam true))

(event Custom|Scale%20Mesh
  (params (NewParam :type Float%20%28single-precision%29))
  (Transformation|SetWorldScale3D (Variables|Character|GetMesh) (Math|Vector|MakeVector 0.0 0.0 NewParam)))

(event EventBeginPlay
  ;[1 1 1] Begin Play
  (CallFunction|ActivateCameras)
  (bind _returnvalue (UserInterface|CreateWidget "/Game/Blueprints/CharacterCreationHUD.CharacterCreationHUD_C" (Game|GetPlayerController 0)))
  (UserInterface|Viewport|AddtoViewport _returnvalue 0))

(event EventTick
  (params (DeltaSeconds :type Float%20%28single-precision%29))
  (bind _vrcamera (Variables|Default|GetVRCamera))
  ;[1 1 1] Event Tick
  (Variables|Default|SetHead%20Rotation (Transformation|GetWorldRotation _vrcamera))
  (Variables|Default|SetHead%20Location (Transformation|GetWorldLocation _vrcamera))
  (CallFunction|AdjustAvatarPositiontoHMDPosition)
  (CallFunction|UpdateAnimBP))

(event Input|KeyboardEvents|Q
  (params (Key :type Key%20Structure :default "AnyKey"))
  ;[1 1 1] adjust camer location
  (:Pressed
    (Variables|Default|SetadjustHeight (+ (Variables|Default|GetadjustHeight) 5.0))))

(event Input|KeyboardEvents|E
  (params (Key :type Key%20Structure :default "AnyKey"))
  ;[1 1 1] adjust camer location
  (:Pressed
    (Variables|Default|SetAdjust%20Sideways (+ (Variables|Default|GetAdjust%20Sideways) 3.0))))

(event Input|KeyboardEvents|R
  (params (Key :type Key%20Structure :default "AnyKey"))
  ;[1 1 1] adjust camer location
  (:Pressed
    (Variables|Default|SetAdjust%20Sideways (+ (Variables|Default|GetAdjust%20Sideways) -3.0))))

(event Input|KeyboardEvents|W
  (params (Key :type Key%20Structure :default "AnyKey"))
  ;[1 1 1] adjust camer location
  (:Pressed
    (Variables|Default|SetadjustHeight (- (Variables|Default|GetadjustHeight) 5.0))))

(event Input|KeyboardEvents|Z
  (params (Key :type Key%20Structure :default "AnyKey"))
  ;[1 1 1] adjust camer location
  (:Pressed
    (Variables|Default|SetAdjust%20Forward (+ (Variables|Default|GetAdjust%20Forward) -3.0))))

(event Input|KeyboardEvents|T
  (params (Key :type Key%20Structure :default "AnyKey"))
  ;[1 1 1] adjust camer location
  (:Pressed
    (Variables|Default|SetAdjust%20Forward (+ (Variables|Default|GetAdjust%20Forward) 3.0))))

(fn ConstructionScript)